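; BP_FloorSwitch is a floor switch that moves itself and a door vertically.
; Four events play or reverse two timelines, whose elevation tracks feed UpdateDoorLocation and UpdateFloorSwitchLocation as Z displacements.
; LowerDoor reverses the door timeline only when SwitchDepressed is false, so the door stays up while the switch is held.
; The graph contains no trigger logic of its own.
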(event EventRaiseDoor
  (bind _doorelevation (Timeline|DoorTimeline Play)
    (:Update
      (Class|FloorSwitch|UpdateDoorLocation (Math|Vector|MakeVector 0.0 0.0 _doorelevation)))))

(event EventLowerDoor
  (if (not (Variables|Default|GetbSwitchDepressed))
    (bind _doorelevation (Timeline|DoorTimeline Reverse)
      (:Update
        (Class|FloorSwitch|UpdateDoorLocation (Math|Vector|MakeVector 0.0 0.0 _doorelevation))))))

(event EventLowerFloorSwitch
  (bind _switchelevation (Timeline|FloorSwitchTimeline Play)
    (:Update
      (Class|FloorSwitch|UpdateFloorSwitchLocation (Math|Vector|MakeVector 0.0 0.0 _switchelevation)))))

(event EventRaiseFloorSwitch
  (bind _switchelevation (Timeline|FloorSwitchTimeline Reverse)
    (:Update
      (Class|FloorSwitch|UpdateFloorSwitchLocation (Math|Vector|MakeVector 0.0 0.0 _switchelevation)))))

(fn ConstructionScript)